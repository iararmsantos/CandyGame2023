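; Side-scroller boss character that chases the player along X, fires projectiles and, on death, marks a level in the save and returns to the main menu.
; Tick handles facing and movement until within range, while a looping timer triggers attack animations and a separate Attack event spawns the aimed projectile.
; Damage updates the boss health bar, knocks it back, jumps animation states and restores Flying movement after a delay.
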(event Custom|HandleRotation
  ;[1 1 1] Handle Rotation
  (if (not (Variables|Default|GetisDead?))
    (if (< (.x (Math|Vector|GetUnitDirection(Vector) (Transformation|GetActorLocation (Game|GetPlayerCharacter 0)) (Transformation|GetActorLocation))) 0.0)
      (Transformation|SetActorRotation "0, 0, 0")
      (else
        (Transformation|SetActorRotation "0.000000,180.000000,0.000000")))))

(event Custom|Boss%20Attack%20Animation
  (if (not (or (Variables|Default|GetisDamaged?) (Variables|Default|GetisDead?)))
    (Class|PaperZDAnimInstance|JumptoNode (Variables|/Script/PaperZD.PaperZDAnimationComponent|GetAnimInstance (Variables|Default|GetAnimationComponent)) "attack" "None")))

(event Custom|Attack
  ;[1 1 1] Handle Attack
  (Transformation|SetWorldRotation (Variables|Default|GetprojectileSpawnLocation) (Math|Rotator|FindLookatRotation (Transformation|GetActorLocation) (Transformation|GetActorLocation (Game|GetPlayerCharacter 0))) false false)
  (Game|SpawnActorfromClass "/Game/Platform/Weapons/BP_BossProjectile.BP_BossProjectile_C" (Transformation|GetWorldTransform (Variables|Default|GetprojectileSpawnLocation)) "Undefined" 0 0))

(event EventBeginPlay
  (Variables|Default|SetmaxHealth (Variables|Default|Gethealth))
  (bind _returnvalue (UserInterface|CreateWidget "/Game/Platform/UI/Widgets/WB_BossHealthBar.WB_BossHealthBar_C" 0 self))
  (bind _output_get (Variables|Default|SetbossHudRef _returnvalue))
  (UserInterface|Viewport|AddtoViewport _output_get 0)
  (bind _returnvalue_2 (Utilities|Time|SetTimerbyEvent (delegate Custom|Boss%20Attack%20Animation) (Math|Random|RandomFloatinRange 2.0 4.0) true))
  (Variables|Default|SetbossAttackEvent _returnvalue_2))

(event Game|Damage|EventAnyDamage
  (params (Damage :type Float%20%28single-precision%29) (DamageType :type Damage%20Type%20Object%20Reference) (InstigatedBy :type Controller%20Object%20Reference) (DamageCauser :type Actor%20Object%20Reference))
  ;[1 1 1] Handle Damage
  (Variables|Default|Sethealth (- (Variables|Default|Gethealth) 1.0))
  (Variables|Default|SetisDamaged? true)
  (Default|UpdateHealthBar (Variables|Default|GetbossHudRef))
  (Character|LaunchCharacter (Math|Vector|MakeVector (* (select (< (.x (Math|Vector|GetUnitDirection(Vector) (Transformation|GetActorLocation DamageCauser) (Transformation|GetActorLocation))) 0.0) 1.0 -1.0) -1e+03) 0.0 0.0) false false)
  (Utilities|FlowControl|Sequence
    (:then_0
      (if (<= (Variables|Default|Gethealth) 0.0)
        (Variables|Default|SetisDead? true)
        (Widget|RemovefromParent (Variables|Default|GetbossHudRef))
        (Class|PaperZDAnimInstance|JumptoNode (Variables|/Script/PaperZD.PaperZDAnimationComponent|GetAnimInstance (Variables|Default|GetAnimationComponent)) "death" "None")
        (Utilities|FlowControl|Delay 2.0)
        (bind _asbp_player_1 (Utilities|Casting|CastToBP_Player1 (Game|GetPlayerCharacter 0)))
        (Utilities|Array|SetArrayElem (Variables|/Game/Platform/Characters/Players/Player1_BP/BP_SaveGame.BP_SaveGame_C|Getlevels (Variables|/Game/Platform/Characters/Players/Player1_BP/BP_Player1.BP_Player1_C|GetsaveGameRef _asbp_player_1)) 2 true)
        (SaveGame|SaveGametoSlot (Variables|/Game/Platform/Characters/Players/Player1_BP/BP_Player1.BP_Player1_C|GetsaveGameRef _asbp_player_1) "1")
        (Game|OpenLevel(byName) "LV_MainMenu")
        (else
          (Class|PaperZDAnimInstance|JumptoNode (Variables|/Script/PaperZD.PaperZDAnimationComponent|GetAnimInstance (Variables|Default|GetAnimationComponent)) "damaged" "None")
          (Utilities|FlowControl|RetriggerableDelay 1.0)
          (Variables|Default|SetisDamaged? false))))
    (:then_1
      (Utilities|FlowControl|Delay 0.7)
      (Pawn|Components|CharacterMovement|SetMovementMode (Variables|Character|GetCharacterMovement) "MOVE_Flying" 0))))

(event EventTick
  (params (DeltaSeconds :type Float%20%28single-precision%29))
  (bind _returnvalue (Transformation|GetActorLocation))
  (bind _returnvalue_2 (Game|GetPlayerCharacter 0))
  (bind _returnvalue_3 (Transformation|GetActorLocation _returnvalue_2))
  (bind _returnvalue_4 (- _returnvalue_3 _returnvalue))
  ;[1 1 1] Handling Movement
  (if (not (Variables|Default|GetisDead?))
    (CallFunction|HandleRotation)
    (if (not (< (Math|Float|Absolute(Float) (.x _returnvalue_4)) 4.5e+02))
      (Pawn|Input|AddMovementInput "1.000000,0.000000,0.000000" (.x (Math|Vector|Normalize (Math|Vector|MakeVector (.x _returnvalue_4) (.y _returnvalue_4) (.z _returnvalue_4)))) false))))

(fn ConstructionScript)