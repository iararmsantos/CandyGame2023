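; Platformer enemy NPC that makes repeated ranged attacks while the player character is inside its Box1 trigger.
; Entering the box starts a looping timer that jumps the animation instance to an attack node, unless the enemy is dead or falling; leaving clears it.
; A separate SpawnProjectile event spawns the projectile class at the spawn point, facing along the actor's rotation.
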(event OnComponentBeginOverlap(Box1)
  (params (OverlappedComponent :type Primitive%20Component%20Object%20Reference) (OtherActor :type Actor%20Object%20Reference) (OtherComp :type Primitive%20Component%20Object%20Reference) (OtherBodyIndex :type Integer) (bFromSweep :type Boolean) (SweepResult :type Hit%20Result%20Structure%20%28by%20ref%29))
  ;[1 1 1] Handle Attack
  (if (== OtherActor (Game|GetPlayerCharacter 0))
    (bind _returnvalue (Utilities|Time|SetTimerbyEvent (delegate Custom|RangedAttack) 1.0 true))
    (Variables|Default|SettimerRef _returnvalue)))

(event OnComponentEndOverlap(Box1)
  (params (OverlappedComponent :type Primitive%20Component%20Object%20Reference) (OtherActor :type Actor%20Object%20Reference) (OtherComp :type Primitive%20Component%20Object%20Reference) (OtherBodyIndex :type Integer))
  (Utilities|Time|ClearandInvalidateTimerbyHandle (Variables|Default|GettimerRef)))

(event Custom|RangedAttack
  ;[1 1 1] Handle Attack
  (if (not (or (Variables|Default|GetisDead?) (AI|Components|NavMovement|IsFalling (Variables|Character|GetCharacterMovement))))
    (Class|PaperZDAnimInstance|JumptoNode (Variables|/Script/PaperZD.PaperZDAnimationComponent|GetAnimInstance (Variables|Default|GetAnimationComponent)) (Variables|Default|GetattackJumpNode) "None")))

(event Custom|Spawn%20Projectile
  ;[1 1 1] Handle Attack
  (Game|SpawnActorfromClass (Variables|Default|GetBP_ProjectileClass) (Math|Transform|MakeTransform (Transformation|GetWorldLocation (Variables|Default|GetspawnPoint)) (Transformation|GetActorRotation) "1.000000,1.000000,1.000000") "Undefined" 0 0))

(event EventBeginPlay
  (|CallParentFunction) ; This node is disabled and will not be called.\nDrag off pins to build functionality.
)

(event Collision|EventActorBeginOverlap
  (params (OtherActor :type Actor%20Object%20Reference))
  (|CallParentFunction OtherActor) ; This node is disabled and will not be called.\nDrag off pins to build functionality.
)

(event EventTick
  (params (DeltaSeconds :type Float%20%28single-precision%29))
  (|CallParentFunction DeltaSeconds) ; This node is disabled and will not be called.\nDrag off pins to build functionality.
)

(fn ConstructionScript
  (|CallParentFunction))