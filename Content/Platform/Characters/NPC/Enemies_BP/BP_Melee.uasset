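; BP_Melee is a melee enemy NPC that walks along the world X axis and faces its direction of travel.
; Each tick it snaps its rotation to one of two opposite facings from the sign of MovementDirection, then feeds that value as the movement input scale.
; The graph holds no attack logic and never changes MovementDirection itself.
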(event Custom|HandleMovement
  (Pawn|Input|AddMovementInput "1.000000,0.000000,0.000000" (Variables|Default|GetmovementDirection) false))

(event Custom|HandleRotation
  (if (> (Variables|Default|GetmovementDirection) 0.0)
    (Transformation|SetActorRotation "0, 0, 0")
    (else
      (Transformation|SetActorRotation "0.000000,180.000000,0.000000"))))

(event EventBeginPlay)

(event Collision|EventActorBeginOverlap
  (params (OtherActor :type Actor%20Object%20Reference)))

(event EventTick
  (params (DeltaSeconds :type Float%20%28single-precision%29))
  (CallFunction|HandleRotation)
  (CallFunction|HandleMovement))

(fn ConstructionScript)