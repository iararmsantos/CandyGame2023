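; Melee enemy character for a side-on platformer that patrols along X and attacks the player.
; Each tick it faces its movement direction and walks, using line traces to pause and turn at walls and ledges.
; A box overlap starts a repeating attack-animation timer, while a separate Attack event traces forward to deal damage.
; Damage updates the health bar widget, turns it toward the attacker, then knocks it back or plays death and destroys it.
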(event OnComponentBeginOverlap(Box)
  (params (OverlappedComponent :type Primitive%20Component%20Object%20Reference) (OtherActor :type Actor%20Object%20Reference) (OtherComp :type Primitive%20Component%20Object%20Reference) (OtherBodyIndex :type Integer) (bFromSweep :type Boolean) (SweepResult :type Hit%20Result%20Structure%20%28by%20ref%29))
  ;[1 1 1] Begin og Attack
  (if (== OtherActor (Game|GetPlayerCharacter 0))
    (Variables|DoNotEdit|SetattackMode? true)
    (bind _returnvalue (Utilities|Time|SetTimerbyEvent (delegate Custom|MeleeAttackEvent) 1.0 true))
    (Variables|DoNotEdit|SetattackEvent _returnvalue)
    (Class|PaperZDAnimInstance|JumptoNode (Variables|/Script/PaperZD.PaperZDAnimationComponent|GetAnimInstance (Variables|Default|GetAnimationComponent)) (Variables|Edit|GetattackJumpNode) "None")))

(event OnComponentEndOverlap(Box)
  (params (OverlappedComponent :type Primitive%20Component%20Object%20Reference) (OtherActor :type Actor%20Object%20Reference) (OtherComp :type Primitive%20Component%20Object%20Reference) (OtherBodyIndex :type Integer))
  ;[1 1 1] End of attack
  (if (== OtherActor (Game|GetPlayerCharacter 0))
    (Variables|DoNotEdit|SetattackMode? false)
    (Utilities|Time|ClearandInvalidateTimerbyHandle (Variables|DoNotEdit|GetattackEvent))))

(event Custom|HandleMovement
  (bind _returnvalue (Transformation|GetActorLocation))
  (bind _returnvalue_2 (Transformation|GetActorLocation))
  ;[1 1 1] Handle Movement
  (if (not (Math|Boolean|ORBoolean (Variables|DoNotEdit|GetisDead?) (Variables|DoNotEdit|GetenemyDamaged?) (Variables|DoNotEdit|GetattackMode?) (AI|Components|NavMovement|IsFalling (Variables|Character|GetCharacterMovement))))
    (Pawn|Input|AddMovementInput "1.000000,0.000000,0.000000" (Variables|DoNotEdit|GetmovementDirection) false)
    (Utilities|FlowControl|Sequence
      (:then_0
        ;;[1 1 1] Check for wall
        (bind _returnvalue_3 (Collision|LineTraceForObjects _returnvalue (+ _returnvalue (* (Transformation|GetActorForwardVector) (Math|Vector|MakeVector 1e+02 0.0 0.0))) (Utilities|Array|MakeArray "ObjectTypeQuery1" "ObjectTypeQuery2" "ObjectTypeQuery3") false (Utilities|Array|MakeArray (Game|GetPlayerCharacter 0)) "ForDuration"))
        (if _returnvalue_3
          (Utilities|FlowControl|DoOnce false :!label _label
            (:Completed
              (Variables|/Script/Engine.CharacterMovementComponent|SetMaxWalkSpeed (Variables|Character|GetCharacterMovement) 0.0)
              (Utilities|FlowControl|Delay (Variables|Edit|GetwaitTime))
              (Variables|/Script/Engine.CharacterMovementComponent|SetMaxWalkSpeed (Variables|Character|GetCharacterMovement) (Variables|Edit|GetenemyWalkSpeed))
              (Variables|DoNotEdit|SetmovementDirection (* (Variables|DoNotEdit|GetmovementDirection) -1.0))
              (goto _label Reset)))))
      (:then_1
        ;;[1 1 1] Check for edges
        (bind _returnvalue_4 (Collision|LineTraceForObjects _returnvalue_2 (+ (- _returnvalue_2 "0.000000,0.000000,100.000000") (* (Transformation|GetActorForwardVector) (Math|Vector|MakeVector 1e+02 0.0 0.0))) (Utilities|Array|MakeArray "ObjectTypeQuery1" "ObjectTypeQuery2" "ObjectTypeQuery3") false (Utilities|Array|MakeArray (Game|GetPlayerCharacter 0)) "None"))
        (if (not _returnvalue_4)
          (goto _label))))))

(event Custom|HandleRotation
  ;[1 1 1] Handle Rotation
  (if (not (Variables|DoNotEdit|GetisDead?))
    (if (> (Variables|DoNotEdit|GetmovementDirection) 0.0)
      (Transformation|SetActorRotation "0, 0, 0")
      (else
        (Transformation|SetActorRotation "0.000000,180.000000,0.000000")))))

(event Custom|MeleeAttackEvent
  ;[1 1 1] Begin og Attack
  (if (not (Variables|DoNotEdit|GetisDead?))
    (bind _returnvalue (Utilities|Time|SetTimerbyEvent (delegate Custom|MeleeAttackEvent) 1.0 true))
    (Variables|DoNotEdit|SetattackEvent _returnvalue)
    (Class|PaperZDAnimInstance|JumptoNode (Variables|/Script/PaperZD.PaperZDAnimationComponent|GetAnimInstance (Variables|Default|GetAnimationComponent)) (Variables|Edit|GetattackJumpNode) "None")))

(event Custom|Attack
  (bind _returnvalue (Transformation|GetActorLocation))
  ;[1 1 1] Attack Event
  (bind _outhit (Collision|LineTraceForObjects _returnvalue (+ _returnvalue (* (Transformation|GetActorForwardVector) (Math|Vector|MakeVector 2e+02 0.0 0.0))) (Utilities|Array|MakeArray "ObjectTypeQuery3") false 0 "ForDuration"))
  (if (== (.HitActor (Collision|BreakHitResult _outhit)) (Game|GetPlayerCharacter 0))
    (Game|Damage|ApplyDamage (.HitActor (Collision|BreakHitResult _outhit)) 1.0 0 0)))

(event EventBeginPlay
  (Variables|/Script/Engine.CharacterMovementComponent|SetMaxWalkSpeed (Variables|Character|GetCharacterMovement) (Variables|Edit|GetenemyWalkSpeed))
  (Variables|DoNotEdit|SetmaxHealth (Variables|Edit|Gethealth))
  (bind _aswb_enemy_health_bar (Utilities|Casting|CastToWB_EnemyHealthBar (UserInterface|GetWidget (Variables|Default|GetWidget))))
  (Variables|/Game/Platform/UI/Widgets/WB_EnemyHealthBar.WB_EnemyHealthBar_C|SetenemyMeleeRef _aswb_enemy_health_bar self)
  (Variables|DoNotEdit|SetWB_EnemyHealthBarRef _aswb_enemy_health_bar))

(event Collision|EventActorBeginOverlap
  (params (OtherActor :type Actor%20Object%20Reference)))

(event EventTick
  (params (DeltaSeconds :type Float%20%28single-precision%29))
  (CallFunction|HandleRotation)
  (CallFunction|HandleMovement))

(event Game|Damage|EventAnyDamage
  (params (Damage :type Float%20%28single-precision%29) (DamageType :type Damage%20Type%20Object%20Reference) (InstigatedBy :type Controller%20Object%20Reference) (DamageCauser :type Actor%20Object%20Reference))
  (bind _returnvalue (Transformation|GetActorLocation DamageCauser))
  (bind _returnvalue_2 (Transformation|GetActorLocation))
  (bind _returnvalue_3 (Math|Vector|GetUnitDirection(Vector) _returnvalue _returnvalue_2))
  (bind _returnvalue_4 (< (.x _returnvalue_3) 0.0))
  (bind _returnvalue_5 (select _returnvalue_4 1.0 -1.0))
  ;[1 1 1] Handle damage
  (Variables|Edit|Sethealth (- (Variables|Edit|Gethealth) Damage))
  (Default|UpdateHealthBar (Variables|DoNotEdit|GetWB_EnemyHealthBarRef))
  (Variables|DoNotEdit|SetenemyDamaged? true)
  (Variables|DoNotEdit|SetmovementDirection _returnvalue_5)
  (if (<= (Variables|Edit|Gethealth) 0.0)
    (Class|PaperZDAnimInstance|JumptoNode (Variables|/Script/PaperZD.PaperZDAnimationComponent|GetAnimInstance (Variables|Default|GetAnimationComponent)) (Variables|Edit|GetdeathJumpNode) "None")
    (Variables|DoNotEdit|SetisDead? true)
    (Rendering|SetVisibility (Variables|Default|GetWidget) false false)
    (Collision|SetCollisionProfileName (Variables|Default|GetCapsuleComponent) "OverlapOnlyPawn" true :!class /Script/Engine.PrimitiveComponent)
    (Utilities|FlowControl|Delay 0.3)
    (Actor|DestroyActor)
    (else
      (Character|LaunchCharacter (Math|Vector|MakeVector (* _returnvalue_5 -8e+02) 0.0 1e+02) true true)
      (Class|PaperZDAnimInstance|JumptoNode (Variables|/Script/PaperZD.PaperZDAnimationComponent|GetAnimInstance (Variables|Default|GetAnimationComponent)) (Variables|Edit|GetdamagedJumpNode) "None")
      (Rendering|SetVisibility (Variables|Default|GetWidget) true false)
      (Utilities|FlowControl|RetriggerableDelay 0.1)
      (Variables|DoNotEdit|SetenemyDamaged? false))))

(fn ConstructionScript)