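; Flying ranged enemy for a side-scrolling platformer that patrols along the X axis and shoots projectiles.
; A forward line trace, ignoring the player, makes it pause and reverse at obstacles.
; Seeing BP_Player1 starts a looping timer that jumps to the attack animation, while a separate event spawns the projectile.
; Damage updates its widget health bar, turns and knocks it back, or plays death before delayed destruction.
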(event OnSeePawn(PawnSensing)
  (params (Pawn :type Pawn%20Object%20Reference))
  ;[1 1 1] Handle Attack
  (Utilities|Casting|CastToBP_Player1 Pawn)
  (Utilities|Time|SetTimerbyEvent (delegate Custom|RangedAttack) 0.6 true))

(event Custom|HandleMovement
  (bind _returnvalue (Transformation|GetActorLocation))
  ;[1 1 1] Handling Movement
  (if (not (or (Variables|Default|GetisDead?) (Variables|Default|GetenemyDamaged?)))
    (Pawn|Input|AddMovementInput "1.000000,0.000000,0.000000" (select (Variables|Default|GetmoveRight) 1.0 -1.0) false)
    (bind _returnvalue_2 (Collision|LineTraceForObjects _returnvalue (+ _returnvalue (* (Transformation|GetActorForwardVector) (Math|Vector|MakeVector 1e+02 0.0 0.0))) (Utilities|Array|MakeArray "ObjectTypeQuery1" "ObjectTypeQuery2" "ObjectTypeQuery3") false (Utilities|Array|MakeArray (Game|GetPlayerCharacter 0)) "ForDuration"))
    (if _returnvalue_2
      (Utilities|FlowControl|DoOnce false :!label _label
        (:Completed
          (Variables|/Script/Engine.CharacterMovementComponent|SetMaxFlySpeed (Variables|Character|GetCharacterMovement) 0.0)
          (Utilities|FlowControl|Delay (Variables|Default|GetwaitTime))
          (Variables|/Script/Engine.CharacterMovementComponent|SetMaxFlySpeed (Variables|Character|GetCharacterMovement) (Variables|Default|GetenemyFlySpeed))
          (Variables|Default|SetmoveRight (not (Variables|Default|GetmoveRight)))
          (goto _label Reset))))))

(event Custom|RangedAttack
  ;[1 1 1] Handle Attack
  (if (not (Variables|Default|GetisDead?))
    (Class|PaperZDAnimInstance|JumptoNode (Variables|/Script/PaperZD.PaperZDAnimationComponent|GetAnimInstance (Variables|Default|GetAnimationComponent)) (Variables|Default|GetattackJumpNode) "None")))

(event Custom|Spawn%20Projectile
  ;[1 1 1] Handle Attack
  (Game|SpawnActorfromClass (Variables|Default|GetProjectileClass) (Math|Transform|MakeTransform (Transformation|GetWorldLocation (Variables|Default|GetspawnPoint)) (Transformation|GetActorRotation) "1.000000,1.000000,1.000000") "Undefined" 0 0))

(event Custom|Handle%20Rotation
  ;[1 1 1] Handling Rotation
  (if (Variables|Default|GetmoveRight)
    (Transformation|SetActorRotation "0, 0, 0")
    (else
      (Transformation|SetActorRotation "0.000000,180.000000,0.000000"))))

(event EventBeginPlay
  (Variables|Default|SetmoveRight (Math|Random|RandomBool))
  (Variables|/Script/Engine.CharacterMovementComponent|SetMaxFlySpeed (Variables|Character|GetCharacterMovement) (Variables|Default|GetenemyFlySpeed))
  (Variables|Default|SetmaxHealth (Variables|Default|Gethealth))
  (bind _aswb_fly_ranged_health_bar (Utilities|Casting|CastToWB_FlyRangedHealthBar (UserInterface|GetWidget (Variables|Default|GetWidget))))
  (Variables|/Game/Platform/UI/Widgets/WB_FlyRangedHealthBar.WB_FlyRangedHealthBar_C|SetenemyRef _aswb_fly_ranged_health_bar self)
  (Variables|Default|SetAs%20WB%20Fly%20Ranged%20Health%20Bar _aswb_fly_ranged_health_bar))

(event EventTick
  (params (DeltaSeconds :type Float%20%28single-precision%29))
  (CallFunction|HandleRotation)
  (CallFunction|HandleMovement))

(event Game|Damage|EventAnyDamage
  (params (Damage :type Float%20%28single-precision%29) (DamageType :type Damage%20Type%20Object%20Reference) (InstigatedBy :type Controller%20Object%20Reference) (DamageCauser :type Actor%20Object%20Reference))
  (bind _returnvalue (Transformation|GetActorLocation DamageCauser))
  (bind _returnvalue_2 (Transformation|GetActorLocation))
  (bind _returnvalue_3 (Math|Vector|GetUnitDirection(Vector) _returnvalue _returnvalue_2))
  (bind _returnvalue_4 (< (.x _returnvalue_3) 0.0))
  (bind _returnvalue_5 (select _returnvalue_4 1.0 0.0))
  ;[1 1 1] Handle damage
  (Variables|Default|Sethealth (- (Variables|Default|Gethealth) Damage))
  (Default|UpdateHealthBar (Variables|Default|GetAs%20WB%20Fly%20Ranged%20Health%20Bar))
  (Variables|Default|SetenemyDamaged? true)
  (Variables|Default|SetmoveRight (> _returnvalue_5 0.0))
  (if (<= (Variables|Default|Gethealth) 0.0)
    (Class|PaperZDAnimInstance|JumptoNode (Variables|/Script/PaperZD.PaperZDAnimationComponent|GetAnimInstance (Variables|Default|GetAnimationComponent)) (Variables|Default|GetdeathJumpNode) "None")
    (Variables|Default|SetisDead? true)
    (Utilities|Time|ClearandInvalidateTimerbyHandle (Variables|Default|GetattackEvent))
    (Rendering|SetVisibility (Variables|Default|GetWidget) false false)
    (Collision|SetCollisionProfileName (Variables|Default|GetCapsuleComponent) "OverlapOnlyPawn" true :!class /Script/Engine.PrimitiveComponent)
    (Utilities|FlowControl|Delay 3.0)
    (Actor|DestroyActor)
    (else
      (Character|LaunchCharacter (Math|Vector|MakeVector (* _returnvalue_5 -8e+02) 0.0 1e+02) true true)
      (Class|PaperZDAnimInstance|JumptoNode (Variables|/Script/PaperZD.PaperZDAnimationComponent|GetAnimInstance (Variables|Default|GetAnimationComponent)) (Variables|Default|GetdamagedJumpNode) "None")
      (Rendering|SetVisibility (Variables|Default|GetWidget) true false)
      (Utilities|FlowControl|RetriggerableDelay 0.1)
      (Variables|Default|SetenemyDamaged? false))))

(fn ConstructionScript)