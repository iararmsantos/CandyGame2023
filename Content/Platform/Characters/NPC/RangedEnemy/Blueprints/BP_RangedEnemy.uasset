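; Ranged enemy for a 2D platformer that faces the player along X, attacks with projectiles and dies when its health runs out.
; Player overlap with its Box starts a looping, never-cleared timer that plays the attack animation unless dead or falling; a separate SpawnProjectile event spawns BP_EnemyProjectile.
; Damage updates the widget health bar, then either applies knockback with a hurt animation or plays death and destroys the actor.
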(event OnComponentBeginOverlap(Box)
  (params (OverlappedComponent :type Primitive%20Component%20Object%20Reference) (OtherActor :type Actor%20Object%20Reference) (OtherComp :type Primitive%20Component%20Object%20Reference) (OtherBodyIndex :type Integer) (bFromSweep :type Boolean) (SweepResult :type Hit%20Result%20Structure%20%28by%20ref%29))
  ;[1 1 1] Handle Attack
  (if (== OtherActor (Game|GetPlayerCharacter 0))
    (Utilities|Time|SetTimerbyEvent (delegate Custom|RangedAttack) 1.0 true)))

(event Custom|HandleRotation
  ;[1 1 1] Handle Rotation
  (if (not (Variables|Default|GetisDead?))
    (if (< (.x (Math|Vector|GetUnitDirection(Vector) (Transformation|GetActorLocation (Game|GetPlayerCharacter 0)) (Transformation|GetActorLocation))) 0.0)
      (Transformation|SetActorRotation "0, 0, 0")
      (else
        (Transformation|SetActorRotation "0.000000,180.000000,0.000000")))))

(event Custom|RangedAttack
  ;[1 1 1] Handle Attack
  (if (not (or (Variables|Default|GetisDead?) (AI|Components|NavMovement|IsFalling (Variables|Character|GetCharacterMovement))))
    (Class|PaperZDAnimInstance|JumptoNode (Variables|/Script/PaperZD.PaperZDAnimationComponent|GetAnimInstance (Variables|Default|GetAnimationComponent)) "attack" "None")))

(event Custom|Spawn%20Projectile
  ;[1 1 1] Handle Attack
  (Game|SpawnActorfromClass "/Game/Platform/Weapons/BP_EnemyProjectile.BP_EnemyProjectile_C" (Math|Transform|MakeTransform (Transformation|GetWorldLocation (Variables|Default|GetspawnPoint)) (Transformation|GetActorRotation) "1.000000,1.000000,1.000000") "Undefined" 0 0))

(event EventBeginPlay
  (Variables|Default|SetmaxHealth (Variables|Default|Gethealth))
  (bind _aswb_ranged_health_bar (Utilities|Casting|CastToWB_RangedHealthBar (UserInterface|GetWidget (Variables|Default|GetWidget))))
  (bind _output_get (Variables|Default|SetAs%20WB%20Ranged%20Health%20Bar _aswb_ranged_health_bar))
  (Variables|/Game/Platform/UI/Widgets/WB_RangedHealthBar.WB_RangedHealthBar_C|SetBP_RangedRef _output_get self))

(event EventTick
  (params (DeltaSeconds :type Float%20%28single-precision%29))
  (CallFunction|HandleRotation))

(event Game|Damage|EventAnyDamage
  (params (Damage :type Float%20%28single-precision%29) (DamageType :type Damage%20Type%20Object%20Reference) (InstigatedBy :type Controller%20Object%20Reference) (DamageCauser :type Actor%20Object%20Reference))
  ;[1 1 1] Handle damage
  (Variables|Default|Sethealth (- (Variables|Default|Gethealth) Damage))
  (Default|UpdateHealthBar (Variables|Default|GetAs%20WB%20Ranged%20Health%20Bar))
  (Variables|Default|SetenemyDamaged? true)
  (if (<= (Variables|Default|Gethealth) 0.0)
    (Class|PaperZDAnimInstance|JumptoNode (Variables|/Script/PaperZD.PaperZDAnimationComponent|GetAnimInstance (Variables|Default|GetAnimationComponent)) "death" "None")
    (Variables|Default|SetisDead? true)
    (Rendering|SetVisibility (Variables|Default|GetWidget) false false)
    (Collision|SetCollisionProfileName (Variables|Default|GetCapsuleComponent) "OverlapOnlyPawn" true :!class /Script/Engine.PrimitiveComponent)
    (Utilities|FlowControl|Delay 0.3)
    (Actor|DestroyActor)
    (else
      (Character|LaunchCharacter (Math|Vector|MakeVector (* (select (< (.x (Math|Vector|GetUnitDirection(Vector) (Transformation|GetActorLocation DamageCauser) (Transformation|GetActorLocation))) 0.0) 1.0 -1.0) -8e+02) 0.0 1e+02) true true)
      (Class|PaperZDAnimInstance|JumptoNode (Variables|/Script/PaperZD.PaperZDAnimationComponent|GetAnimInstance (Variables|Default|GetAnimationComponent)) "damaged" "None")
      (Rendering|SetVisibility (Variables|Default|GetWidget) true false)
      (Utilities|FlowControl|RetriggerableDelay 0.1)
      (Variables|Default|SetenemyDamaged? false))))

(fn ConstructionScript)