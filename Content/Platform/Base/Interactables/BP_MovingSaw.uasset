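; BP_MovingSaw is a platformer saw hazard that moves between two points and damages the player on contact.
; The construction script feeds relative Location1 and Location2 into InterpToMovement as control points, with Speed as the travel Duration.
; Sphere overlap with BP_Player1 applies damage and launches the player.
; Both MoveRight branches launch along positive X, so the knockback ignores facing.
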(event OnComponentBeginOverlap(Sphere)
  (params (OverlappedComponent :type Primitive%20Component%20Object%20Reference) (OtherActor :type Actor%20Object%20Reference) (OtherComp :type Primitive%20Component%20Object%20Reference) (OtherBodyIndex :type Integer) (bFromSweep :type Boolean) (SweepResult :type Hit%20Result%20Structure%20%28by%20ref%29))
  (bind _asbp_player_1 (Utilities|Casting|CastToBP_Player1 OtherActor))
  (Game|Damage|ApplyDamage OtherActor 1.0 0 self)
  (if (Variables|/Game/Platform/Characters/Players/Player1_BP/BP_Player1.BP_Player1_C|GetmoveRight? _asbp_player_1)
    (Character|LaunchCharacter _asbp_player_1 "1000.000000,0.000000,0.000000" false false)
    (else
      (Character|LaunchCharacter _asbp_player_1 "1000.000000,0.000000,0.000000" false false))))

(fn ConstructionScript
  (bind _interptomovement (Variables|Default|GetInterpToMovement))
  (Variables|/Script/Engine.InterpToMovementComponent|SetControlPoints _interptomovement (Utilities|Array|MakeArray (Utilities|Struct|MakeInterpControlPoint (Variables|Default|Getlocation1) true) (Utilities|Struct|MakeInterpControlPoint (Variables|Default|Getlocation2) true)))
  (Variables|/Script/Engine.InterpToMovementComponent|SetDuration _interptomovement (Variables|Default|Getspeed)))