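; BP_CoinsPickup is a collectible coin that the player picks up by overlapping its Sphere component.
; The overlap casts to BP_Player1, adds one to its Coins, refreshes the coin HUD and destroys the pickup.
; If Coins already equals exactly 100, it instead resets Coins to zero, adds a life and updates only the lives HUD before destroying itself.
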(event OnComponentBeginOverlap(Sphere)
  (params (OverlappedComponent :type Primitive%20Component%20Object%20Reference) (OtherActor :type Actor%20Object%20Reference) (OtherComp :type Primitive%20Component%20Object%20Reference) (OtherBodyIndex :type Integer) (bFromSweep :type Boolean) (SweepResult :type Hit%20Result%20Structure%20%28by%20ref%29))
  (bind _asbp_player_1 (Utilities|Casting|CastToBP_Player1 OtherActor))
  (Variables|Default|SetBP_Player%201Ref _asbp_player_1)
  (if (== (Variables|/Game/Platform/Characters/Players/Player1_BP/BP_Player1.BP_Player1_C|Getcoins _asbp_player_1) 1e+02)
    (Variables|/Game/Platform/Characters/Players/Player1_BP/BP_Player1.BP_Player1_C|Setcoins (Variables|Default|GetBP_Player%201Ref) 0.0)
    (Variables|/Game/Platform/Characters/Players/Player1_BP/BP_Player1.BP_Player1_C|Setlives (Variables|Default|GetBP_Player%201Ref) (+ (Variables|/Game/Platform/Characters/Players/Player1_BP/BP_Player1.BP_Player1_C|Getlives (Variables|Default|GetBP_Player%201Ref)) 1.0))
    (Default|UpdateLives (Variables|/Game/Platform/Characters/Players/Player1_BP/BP_Player1.BP_Player1_C|GethudRef (Variables|Default|GetBP_Player%201Ref)))
    (Actor|DestroyActor)
    (else
      (Variables|/Game/Platform/Characters/Players/Player1_BP/BP_Player1.BP_Player1_C|Setcoins (Variables|Default|GetBP_Player%201Ref) (+ (Variables|/Game/Platform/Characters/Players/Player1_BP/BP_Player1.BP_Player1_C|Getcoins (Variables|Default|GetBP_Player%201Ref)) 1.0))
      (Default|UpdateCoins (Variables|/Game/Platform/Characters/Players/Player1_BP/BP_Player1.BP_Player1_C|GethudRef (Variables|Default|GetBP_Player%201Ref)))
      (Actor|DestroyActor))))

(event EventBeginPlay)

(event Collision|EventActorBeginOverlap
  (params (OtherActor :type Actor%20Object%20Reference)))

(event EventTick
  (params (DeltaSeconds :type Float%20%28single-precision%29)))

(fn ConstructionScript)