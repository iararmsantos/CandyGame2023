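; BP_HealthPickup is a collectible that restores health to BP_Player1 when it enters the pickup's sphere.
; Every player overlap plays the Heal sound, even at full health, when the pickup otherwise stays in place.
; Below full health, it adds HealthToGive clamped to MaxHealth, passes the truncated, unclamped HealthToGive to the HUD's ShowHearts, then destroys itself.
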(event OnComponentBeginOverlap(Sphere)
  (params (OverlappedComponent :type Primitive%20Component%20Object%20Reference) (OtherActor :type Actor%20Object%20Reference) (OtherComp :type Primitive%20Component%20Object%20Reference) (OtherBodyIndex :type Integer) (bFromSweep :type Boolean) (SweepResult :type Hit%20Result%20Structure%20%28by%20ref%29))
  (bind _asbp_player_1 (Utilities|Casting|CastToBP_Player1 OtherActor))
  (Variables|Default|SetBPPlayerRef _asbp_player_1)
  (Audio|PlaySoundatLocation "/Game/Platform/Effects/Sounds/heal.heal" (Transformation|GetActorLocation) "0, 0, 0" 1.0 1.0 0.0 0 0 0 0)
  (if (not (== (Variables|/Game/Platform/Characters/Players/Player1_BP/BP_Player1.BP_Player1_C|Gethealth _asbp_player_1) (Variables|/Game/Platform/Characters/Players/Player1_BP/BP_Player1.BP_Player1_C|GetmaxHealth _asbp_player_1)))
    (Variables|/Game/Platform/Characters/Players/Player1_BP/BP_Player1.BP_Player1_C|Sethealth (Variables|Default|GetBPPlayerRef) (Math|Float|Clamp(Float) (+ (Variables|/Game/Platform/Characters/Players/Player1_BP/BP_Player1.BP_Player1_C|Gethealth (Variables|Default|GetBPPlayerRef)) (Variables|Default|GethealthToGive)) 0.0 (Variables|/Game/Platform/Characters/Players/Player1_BP/BP_Player1.BP_Player1_C|GetmaxHealth (Variables|Default|GetBPPlayerRef))))
    (Default|ShowHearts (Variables|/Game/Platform/Characters/Players/Player1_BP/BP_Player1.BP_Player1_C|GethudRef (Variables|Default|GetBPPlayerRef)) (Math|Float|Truncate (Variables|Default|GethealthToGive)))
    (Actor|DestroyActor)))

(event EventBeginPlay)

(event Collision|EventActorBeginOverlap
  (params (OtherActor :type Actor%20Object%20Reference)))

(event EventTick
  (params (DeltaSeconds :type Float%20%28single-precision%29)))

(fn ConstructionScript)