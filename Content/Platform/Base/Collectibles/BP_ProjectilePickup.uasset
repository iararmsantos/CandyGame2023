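; BP_ProjectilePickup is a collectible that refills the player's projectile ammo.
; When BP_Player1 overlaps its sphere while not at maximum, it adds a fixed amount clamped to the player's limit.
; It then writes the count to the player's save game, saves the slot immediately, refreshes the HUD and destroys itself.
; At full ammo the pickup stays in the world.
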(event OnComponentBeginOverlap(Sphere)
  (params (OverlappedComponent :type Primitive%20Component%20Object%20Reference) (OtherActor :type Actor%20Object%20Reference) (OtherComp :type Primitive%20Component%20Object%20Reference) (OtherBodyIndex :type Integer) (bFromSweep :type Boolean) (SweepResult :type Hit%20Result%20Structure%20%28by%20ref%29))
  (bind _asbp_player_1 (Utilities|Casting|CastToBP_Player1 OtherActor))
  (Variables|Default|SetBPPlayerRef _asbp_player_1)
  (if (not (== (Variables|/Game/Platform/Characters/Players/Player1_BP/BP_Player1.BP_Player1_C|Getprojectile _asbp_player_1) (Variables|/Game/Platform/Characters/Players/Player1_BP/BP_Player1.BP_Player1_C|GetmaxProjectiles _asbp_player_1)))
    (bind _output_get (Variables|/Game/Platform/Characters/Players/Player1_BP/BP_Player1.BP_Player1_C|Setprojectile (Variables|Default|GetBPPlayerRef) (Math|Integer|Clamp(Integer) (+ (Variables|/Game/Platform/Characters/Players/Player1_BP/BP_Player1.BP_Player1_C|Getprojectile (Variables|Default|GetBPPlayerRef)) 5) 1 (Variables|/Game/Platform/Characters/Players/Player1_BP/BP_Player1.BP_Player1_C|GetmaxProjectiles (Variables|Default|GetBPPlayerRef)))))
    (Variables|/Game/Platform/Characters/Players/Player1_BP/BP_SaveGame.BP_SaveGame_C|Setprojectile (Variables|/Game/Platform/Characters/Players/Player1_BP/BP_Player1.BP_Player1_C|GetsaveGameRef (Variables|Default|GetBPPlayerRef)) (Math|Conversions|ToFloat(Integer) _output_get))
    (SaveGame|SaveGametoSlot (Variables|/Game/Platform/Characters/Players/Player1_BP/BP_Player1.BP_Player1_C|GetsaveGameRef (Variables|Default|GetBPPlayerRef)) "1")
    (Default|UpdateProjectiles (Variables|/Game/Platform/Characters/Players/Player1_BP/BP_Player1.BP_Player1_C|GethudRef (Variables|Default|GetBPPlayerRef)))
    (Actor|DestroyActor)))

(event EventBeginPlay)

(event Collision|EventActorBeginOverlap
  (params (OtherActor :type Actor%20Object%20Reference)))

(event EventTick
  (params (DeltaSeconds :type Float%20%28single-precision%29)))

(fn ConstructionScript)